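; BP_CaptureSprite is a TextureToSkeletalMesh tool actor that renders a set of paper sprites into a render target.
; Its construction script spawns one sprite component per entry, rotated flat in a grid whose column count derives from the spacing.
; CaptureSpritesToRT scene-captures only this actor into a transparent temporary target.
; A dynamic material instance then draws that capture into the cleared output render target.
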(fn ConstructionScript
  (Variables|Default|SetColumn (Math|Float|Truncate (/ 1024.0 (Variables|Default|GetSpace))))
  (CallFunction|DisplaySprites))

(fn DisplaySprites
  (for (_array_element _array_index) (Variables|Default|GetSprites)
    (LocalVariables|SetIndex _array_index)
    (bind _returnvalue (AddComponent|AddPaperSpriteComponent false (Math|Transform|MakeTransform (+ (Math|Vector|MakeVector (* (Variables|Default|GetSpace) (.Remainder (Math|Float|Division(WholeandRemainder) (Math|Conversions|ToFloat(Integer) (LocalVariables|GetIndex)) (Math|Conversions|ToFloat(Integer) (Variables|Default|GetColumn))))) (* (.ReturnValue (Math|Float|Division(WholeandRemainder) (Math|Conversions|ToFloat(Integer) (LocalVariables|GetIndex)) (Math|Conversions|ToFloat(Integer) (Variables|Default|GetColumn)))) (Variables|Default|GetSpace)) 0.0) (Math|Vector|MakeVector (* (Variables|Default|GetSpace) (Math|Conversions|ToFloat(Integer) (- (Variables|Default|GetColumn) 1)) -0.5) (* (Math|Conversions|ToFloat(Integer) (.ReturnValue (Math|Float|Division(WholeandRemainder) (Math|Conversions|ToFloat(Integer) (Utilities|Array|Length (Variables|Default|GetSprites))) (Math|Conversions|ToFloat(Integer) (Variables|Default|GetColumn))))) (Variables|Default|GetSpace) -0.5) 0.0)) "0.000000, 0,-90.000000" "1.000000,1.000000,1.000000")))
    (Rendering|Components|Sprite|SetSprite _returnvalue _array_element)))

(fn CaptureSpritestoRT
  (bind _render_target (Variables|Default|GetRender%20Target))
  (Utilities|IsValid (Variables|Default|GetRender%20Target)
    (:Is%20Valid
      ;[1 1 1] Create RT for SceneCaptureComponent2D
      (bind _returnvalue (Rendering|CreateRenderTarget2D (Variables|/Script/Engine.TextureRenderTarget2D|GetSizeX _render_target) (Variables|/Script/Engine.TextureRenderTarget2D|GetSizeY _render_target) "RTF_RGBA16f" "(R=0.000000,G=0.000000,B=0.000000,A=0.000000)"))
      (bind _output_get (LocalVariables|SetTempRT _returnvalue))
      (Variables|/Script/Engine.SceneCaptureComponent2D|SetTextureTarget (Variables|Default|GetSceneCaptureComponent2D) _output_get)
      (bind _returnvalue_2 (Rendering|Material|CreateDynamicMaterialInstance (Variables|Default|GetM_Parent) "None" "None" :!class /Script/Engine.KismetMaterialLibrary))
      (bind _output_get_2 (LocalVariables|SetDMI _returnvalue_2))
      (Rendering|Material|SetTextureParameterValue _output_get_2 "RT" (LocalVariables|GetTempRT))
      (Rendering|SceneCapture|ShowOnlyActorComponents (Variables|Default|GetSceneCaptureComponent2D) self true)
      (Rendering|SceneCapture|CaptureScene (Variables|Default|GetSceneCaptureComponent2D) :!class /Script/Engine.SceneCaptureComponent2D)
      (Rendering|ClearRenderTarget2D (Variables|Default|GetRender%20Target) "(R=0.000000,G=0.000000,B=0.000000,A=0.000000)")
      (Rendering|DrawMaterialtoRenderTarget (Variables|Default|GetRender%20Target) (LocalVariables|GetDMI)))))