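; Animation2DDataAsset is a data asset that describes named animations as frame ranges, apparently for texture-based 2D animation.
; FillAnimationFrameInfoByNameFrameMap clears and rebuilds TextureAnimationInfo from NameFrameMap, which pairs each animation name with a frame count.
; It lays the animations end to end in map order, starting each range one frame after the previous inclusive EndFrame.
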(fn FillAnimationFrameInfobyNameFrameMap
  (Utilities|Array|Clear (Variables|AnimationData|GetTextureAnimationInfo))
  (Utilities|FlowControl|Sequence
    (:then_0
      (bind _keys (Utilities|Map|Keys (Variables|HelperTool|GetNameFrameMap)))
      (LocalVariables|SetNames _keys)
      (bind _values (Utilities|Map|Values (Variables|HelperTool|GetNameFrameMap)))
      (LocalVariables|SetValus _values))
    (:then_1
      (for _index (range 0 (- (Utilities|Array|Length (LocalVariables|GetNames)) 1))
        (LocalVariables|SetIndex _index)
        (LocalVariables|SetStart (+ (LocalVariables|GetEnd) (select (== (LocalVariables|GetIndex) 0) 0 1)))
        (LocalVariables|SetEnd (- (+ (LocalVariables|GetStart) (Utilities|Array|Get(acopy) (LocalVariables|GetValus) (LocalVariables|GetIndex))) 1))
        (Utilities|Array|SetArrayElem (Variables|AnimationData|GetTextureAnimationInfo) (LocalVariables|GetIndex) (Utilities|Struct|MakeS_AnimationData (Utilities|Array|Get(acopy) (LocalVariables|GetNames) (LocalVariables|GetIndex)) (LocalVariables|GetStart) (LocalVariables|GetEnd)) true)))))