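; BP_ExamplePlayer is the playable character for the TextureToSkeletalMesh showcase, with side-scroller style movement on a single axis.
; Enhanced Input drives movement along the world forward vector and jumping, while Tick snaps yaw to face the direction of travel.
; Right mouse spawns a Shoot actor at an offset from the character.
; The attack input is empty, and dash, slide and attack montage chains are left unconnected.
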(event Input|EnhancedActionEvents|EnhancedInputActionIA_Move
  (params (ActionValue :type Float%20%28double-precision%29) (ElapsedSeconds :type Float%20%28double-precision%29) (TriggeredSeconds :type Float%20%28double-precision%29) (InputAction :type Input%20Action%20Object%20Reference :default "/Game/TextureToSkeletalMesh/Showcase/Inputs/InputActions/IA_Move.IA_Move"))
  (Pawn|Input|AddMovementInput (Class|KismetMathLibrary|VectorForward) ActionValue false))

(event Input|EnhancedActionEvents|EnhancedInputActionIA_Attack
  (params (ActionValue :type Boolean) (ElapsedSeconds :type Float%20%28double-precision%29) (TriggeredSeconds :type Float%20%28double-precision%29) (InputAction :type Input%20Action%20Object%20Reference :default "/Game/TextureToSkeletalMesh/Showcase/Inputs/InputActions/IA_Attack.IA_Attack")))

(event Input|EnhancedActionEvents|EnhancedInputActionIA_Jump
  (params (ActionValue :type Boolean) (ElapsedSeconds :type Float%20%28double-precision%29) (TriggeredSeconds :type Float%20%28double-precision%29) (InputAction :type Input%20Action%20Object%20Reference :default "/Game/TextureToSkeletalMesh/Showcase/Inputs/InputActions/IA_Jump.IA_Jump"))
  (:Started
    (Character|Jump))
  (:Completed
    (Character|StopJumping)))

(event EventBeginPlay
  (bind _returnvalue (Game|GetPlayerController 0))
  (bind _returnvalue_2 (PlayerController|LocalPlayerSubsystems|GetEnhancedInputLocalPlayerSubsystem _returnvalue))
  (Utilities|IsValid _returnvalue_2
    (:Is%20Valid
      (Input|AddMappingContext _returnvalue_2 "/Game/TextureToSkeletalMesh/Showcase/Inputs/IMC_Default.IMC_Default" 0 "(bIgnoreAllPressedKeysUntilRelease=True,bForceImmediately=False,bNotifyUserSettings=False)"))))

(event EventTick
  (params (DeltaSeconds :type Float%20%28single-precision%29))
  (bind _returnvalue (Class|KismetMathLibrary|VectorForward))
  (bind _charactermovement (Variables|Character|GetCharacterMovement))
  (bind _velocity (Variables|/Script/Engine.MovementComponent|GetVelocity _charactermovement))
  (bind _returnvalue_2 (Math|Vector|DotProduct _velocity _returnvalue))
  ;[1 0.0409 0] Test rotation
  (if (!= _returnvalue_2 0.0)
    (Transformation|SetActorRotation (Math|Rotator|MakeRotator 0.0 0.0 (select (> _returnvalue_2 0.0) 0.0 1.8e+02)))))

(event Input|KeyboardEvents|Q
  (params (Key :type Key%20Structure :default "None")))

(event Input|MouseEvents|RightMouseButton
  (params (Key :type Key%20Structure :default "None")))

(event Input|MouseEvents|RightMouseButton
  (params (Key :type Key%20Structure :default "None"))
  (bind _returnvalue (Transformation|GetActorLocation))
  (:Pressed
    (Game|SpawnActorfromClass "/Game/TextureToSkeletalMesh/Showcase/Blueprints/shoot.shoot_C" (Math|Transform|MakeTransform (Math|Vector|MakeVector (+ (.x _returnvalue) 5e+01) (.y _returnvalue) (+ (.z _returnvalue) -5e+01)) "0, 0, 0" "1.000000,1.000000,1.000000") "AlwaysSpawn" "OverrideRootScale" 0 0)))

(fn ConstructionScript)